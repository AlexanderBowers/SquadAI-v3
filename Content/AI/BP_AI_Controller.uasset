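; AI controller for squad combat pawns that runs a basic behavior tree and seeds blackboard health by pawn class, a death flag and a Red team.
; Perception updates compare blackboard teams and store enemies as TargetActor.
; Non-AI actors resolve to the squad player controller, hostile when this AI is Red.
; A muzzle-alignment step traces from a Commando's muzzle toward the target, but the hit result drives nothing further.
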(event `self.ReceiveBeginPlay`
  (bind _returnvalue (`AIBlueprintHelperLibrary.GetBlackboard` self))
  (`self.RunBehaviorTree` "/Game/AI/BT_Basic.BT_Basic")
  (cast `/Game/AI/BP_AI_Character_Super` (`self.K2_GetPawn` self)
    (:`then`
      (`BlackboardComponent.SetValueAsFloat` _returnvalue "Health" 100.0))
    (:`CastFailed`
      (`BlackboardComponent.SetValueAsFloat` _returnvalue "Health" 50.0)))
  (`BlackboardComponent.SetValueAsBool` _returnvalue "IsDead" false)
  (`BlackboardComponent.SetValueAsString` _returnvalue "Team" "Red"))

(event `self.AIPerception.OnTargetPerceptionUpdated`
  (params (Actor :type "Actor Object Reference") (Stimulus :type "AIStimulus Structure"))
  (bind (_isenemyteam _enemyai) (`self.IsEnemyTeam?` Actor))
  (if _isenemyteam
    (`self.SetTargetActor` _enemyai)
    (`self.AlignMuzzle`)))

(fn `AlignMuzzle`
  (bind _asbp_commando (cast `/Game/AI/BP_Commando` (`self.K2_GetPawn`)))
  (bind _asbp_ai_character (cast `/Game/AI/BP_AI_Character` (`BlackboardComponent.GetValueAsObject` (`AIBlueprintHelperLibrary.GetBlackboard` null) "TargetActor")))
  (bind _hitlocation (`PrimitiveComponent.K2_LineTraceComponent` (`Character.Mesh` _asbp_commando) (`SceneComponent.K2_GetComponentLocation` (`/Game/AI/BP_AI_Character.Muzzle` _asbp_commando)) (`self.K2_GetActorLocation` _asbp_ai_character) true false false))
  (set `self.Hit Location` _hitlocation))

(fn `GetTargetActor`
  (returns (TargetActor :type "/Game/AI/BP_AI_Character Object Reference"))
  (bind _asbp_ai_character (cast `/Game/AI/BP_AI_Character` (`BlackboardComponent.GetValueAsObject` (`AIBlueprintHelperLibrary.GetBlackboard` self) "TargetActor")))
  (return _asbp_ai_character))

(fn `IsEnemyTeam?`
  (params (Enemy :type "Object Object Reference"))
  (returns (ISEnemyTeam :type Boolean) (EnemyAI :type "Actor Object Reference"))
  (bind _asbp_ai_character (cast `/Game/AI/BP_AI_Character` Enemy)
    (:`then`
      (return (`KismetStringLibrary.NotEqual_StrStr` (`BlackboardComponent.GetValueAsString` (`AIBlueprintHelperLibrary.GetBlackboard` self) "Team") (`BlackboardComponent.GetValueAsString` (`AIBlueprintHelperLibrary.GetBlackboard` _asbp_ai_character) "Team")) _asbp_ai_character))
    (:`CastFailed`
      (bind _asbp_squad_player_controller (cast `/Game/BP_SquadPlayerController` (`GameplayStatics.GetPlayerController` 0)))
      (return (`KismetStringLibrary.EqualEqual_StrStr` (`BlackboardComponent.GetValueAsString` (`AIBlueprintHelperLibrary.GetBlackboard` self) "Team") "Red") _asbp_squad_player_controller))))

(fn `IsTargetActorSet`
  (returns (TargetActor :type "/Game/AI/BP_AI_Character Object Reference") (IsTargetActorSet :type Boolean))
  (bind _returnvalue (`BlackboardComponent.GetValueAsObject` (`AIBlueprintHelperLibrary.GetBlackboard` self) "TargetActor"))
  (bind _asbp_ai_character (cast `/Game/AI/BP_AI_Character` _returnvalue))
  (return _asbp_ai_character (`KismetSystemLibrary.IsValid` _returnvalue)))

(fn `SetTargetActor`
  (params (TheTargetActor :type "Actor Object Reference"))
  (returns (TargetActor :type "Actor Object Reference"))
  (`BlackboardComponent.SetValueAsObject` (`AIBlueprintHelperLibrary.GetBlackboard` self) "TargetActor" TheTargetActor)
  (return TheTargetActor))

(fn `UserConstructionScript`)