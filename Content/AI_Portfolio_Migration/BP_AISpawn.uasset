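; BP_AISpawn is a spawner that keeps one BP_AI_Character in the world at its own location and rotation.
; On BeginPlay it spawns the AI with the BT_Basic behavior tree and writes its Team string into the AI's blackboard.
; Tick checks whether that AI is still valid and, if not, loops back to the same spawn logic after a short delay.
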(event `self.ReceiveBeginPlay`
  (bind _returnvalue (`AIBlueprintHelperLibrary.SpawnAIFromClass` "/Game/AI_Portfolio_Migration/BP_AI_Character.BP_AI_Character_C" "/Game/AI_Portfolio_Migration/BT_Basic.BT_Basic" (`self.K2_GetActorLocation` self) (`self.K2_GetActorRotation` self) false null :!label _label))
  (`BlackboardComponent.SetValueAsString` (`AIBlueprintHelperLibrary.GetBlackboard` _returnvalue) "Team" (`self.Team`)))

(event `self.ReceiveTick`
  (params (DeltaSeconds :type "Float (single-precision)"))
  (if (not (`KismetSystemLibrary.IsValid` (stale `self.ReceiveBeginPlay` _returnvalue)))
    (`KismetSystemLibrary.Delay` 5.0)
    (goto _label)))

(fn `NewFunction_0`)

(fn `UserConstructionScript`)