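; BP_Commando is a commando character Blueprint that automatically crouches while inside designated trigger volumes.
; On overlap begin and end, it casts the other actor to TriggerVolume and matches its display name against "CrouchVolume".
; A match calls Crouch or UnCrouch and updates the IsCrouching flag.
; The volume is identified by name string, and BeginPlay and Tick are disabled.
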(event `self.ReceiveActorBeginOverlap`
  (params (OtherActor :type "Actor Object Reference"))
  (`parent.ReceiveActorBeginOverlap` OtherActor)
  (bind _astrigger_volume (cast `TriggerVolume` OtherActor))
  (if (`KismetStringLibrary.EqualEqual_StrStr` "CrouchVolume" (`KismetSystemLibrary.GetDisplayName` _astrigger_volume))
    (`self.Crouch`)
    (set `self.IsCrouching` true)))

(event `self.ReceiveActorEndOverlap`
  (params (OtherActor :type "Actor Object Reference"))
  (bind _astrigger_volume (cast `TriggerVolume` OtherActor))
  (if (`KismetStringLibrary.EqualEqual_StrStr` "CrouchVolume" (`KismetSystemLibrary.GetDisplayName` _astrigger_volume))
    (`self.UnCrouch`)
    (set `self.IsCrouching` false)))

(fn `UserConstructionScript`
  (`parent.UserConstructionScript`))