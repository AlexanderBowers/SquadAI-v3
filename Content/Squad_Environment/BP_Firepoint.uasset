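; BP_Firepoint is a squad environment position that a squad member can be assigned to through a command point.
; CheckAssignedMember acts as a toggle: it resets the current member's priority command and clears it, or requests an available member from SquadPlayerController using the EndLocation position.
; The chosen member's Blackboard receives this actor as AssignedPosition and is flagged as assigned.
; ResetAssignedMember only clears the stored reference, printing a debug message when none is valid.
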(event `SquadInterface.CheckAssignedMember`
  (params (CommandPoint :type "CommandPoint Structure"))
  (bind (_location _type _owneractor) (break `CommandPoint` CommandPoint))
  (`/Engine/EditorBlueprintResources/StandardMacros.IsValid` (`self.AssignedSquadMember`)
    (:`Is Valid`
      (`SquadAIController.ResetPriorityCommand` (`self.AssignedSquadMember`))
      (set `self.AssignedSquadMember` null))
    (:`Is Not Valid`
      (bind _assquad_player_controller (cast `SquadPlayerController` (`GameplayStatics.GetPlayerController` 0)))
      (bind _returnvalue (`SquadPlayerController.GetAvailableMember` _assquad_player_controller (make `CommandPoint` (`SceneComponent.K2_GetComponentLocation` (`self.EndLocation`)) _type _owneractor)))
      (bind _blackboard (`AIController.Blackboard` _returnvalue))
      (`BlackboardComponent.SetValueAsObject` _blackboard "AssignedPosition" self)
      (`BlackboardComponent.SetValueAsBool` _blackboard "bIsAssigned" true)
      (set `self.AssignedSquadMember` _returnvalue))))

(event `SquadInterface.ResetAssignedMember`
  (`/Engine/EditorBlueprintResources/StandardMacros.IsValid` (`self.AssignedSquadMember`)
    (:`Is Valid`
      (set `self.AssignedSquadMember` null))
    (:`Is Not Valid`
      (`KismetSystemLibrary.PrintString` "Reset Called but not valid."))))

(event `self.ReceiveTick`
  (params (DeltaSeconds :type "Float (single-precision)")))

(fn `UserConstructionScript`)