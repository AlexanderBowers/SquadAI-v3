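; BP_Door is a breachable squad door that squad members blow open with a planted bomb.
; CheckAssignedMember asks BP_SquadPlayerController for available members for the bomb point and two assist points.
; When the first member overlaps Box, a one-time, delay-timed sequence retreats them, spawns and detonates BP_Bomb, destroys both doors and sends all three to exit points.
; Overlaps at Assist1 and EndLocation snap actor facing; OpenDoor applies only a zero offset.
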(event `SquadInterface.CheckAssignedMember`
  (params (CommandPoint :type "CommandPoint Structure"))
  (bind (_location _type _owneractor) (break `CommandPoint` CommandPoint))
  (bind _asbp_squad_player_controller (cast `/Game/AI_Portfolio_Migration/BP_SquadPlayerController` (`GameplayStatics.GetPlayerController` 0)))
  (bind _returnvalue (`SquadPlayerController.GetAvailableMember` _asbp_squad_player_controller (make `CommandPoint` (`SceneComponent.K2_GetComponentLocation` (`self.BombLocation`)) _type _owneractor)))
  (set `self.AssignedSquadMember1` _returnvalue)
  (`KismetSystemLibrary.Delay` 0.1)
  (bind _returnvalue_2 (`SquadPlayerController.GetAvailableMember` _asbp_squad_player_controller (make `CommandPoint` (`SceneComponent.K2_GetComponentLocation` (`self.Assist1`)) _type _owneractor)))
  (set `self.AssignedSquadMember2` _returnvalue_2)
  (`KismetSystemLibrary.Delay` 0.1)
  (bind _returnvalue_3 (`SquadPlayerController.GetAvailableMember` _asbp_squad_player_controller (make `CommandPoint` (`SceneComponent.K2_GetComponentLocation` (`self.Assist2`)) _type _owneractor)))
  (set `self.AssignedSquadMember3` _returnvalue_3))

(event `self.Box.OnComponentBeginOverlap`
  (params (OverlappedComponent :type "PrimitiveComponent Object Reference") (OtherActor :type "Actor Object Reference") (OtherComp :type "PrimitiveComponent Object Reference") (OtherBodyIndex :type Integer) (bFromSweep :type Boolean) (SweepResult :type "HitResult Structure (by ref)"))
  (bind _assignedsquadmember1 (`self.AssignedSquadMember1`))
  (if (== OtherActor (`Controller.K2_GetPawn` _assignedsquadmember1))
    (if (not (`self.IsPlanted`))
      (set `self.IsPlanted` true)
      (`KismetSystemLibrary.Delay` 1.0)
      (`AIController.MoveToLocation` _assignedsquadmember1 (`SceneComponent.K2_GetComponentLocation` (`self.EndLocation`)) -1.0 true true false true null true)
      (bind _returnvalue (`|SpawnActorFromClass` "/Game/BP_Bomb.BP_Bomb_C" (`SceneComponent.K2_GetComponentToWorld` (`self.BombLocation`)) "Undefined" "OverrideRootScale" null null))
      (`KismetSystemLibrary.Delay` 3.0)
      (`/Game/BP_Bomb.Explode` _returnvalue)
      (`ActorComponent.K2_DestroyComponent` (`self.Door`))
      (`ActorComponent.K2_DestroyComponent` (`self.Door2`))
      (`KismetSystemLibrary.Delay` 1.0)
      (`AIController.MoveToLocation` (`self.AssignedSquadMember2`) (`SceneComponent.K2_GetComponentLocation` (`self.ExitLocation`)) 20.0 true true false true null true)
      (`AIController.MoveToLocation` (`self.AssignedSquadMember3`) (`SceneComponent.K2_GetComponentLocation` (`self.ExitLocation2`)) 20.0 true true false true null true)
      (`KismetSystemLibrary.Delay` 0.3)
      (`AIController.MoveToLocation` (`self.AssignedSquadMember1`) (`SceneComponent.K2_GetComponentLocation` (`self.ExitLocation3`)) 20.0 true true false true null true))))

(event `self.Assist1.OnComponentBeginOverlap`
  (params (OverlappedComponent :type "PrimitiveComponent Object Reference") (OtherActor :type "Actor Object Reference") (OtherComp :type "PrimitiveComponent Object Reference") (OtherBodyIndex :type Integer) (bFromSweep :type Boolean) (SweepResult :type "HitResult Structure (by ref)"))
  (`self.K2_SetActorRotation` OtherActor (struct :`Yaw` 90.0) false))

(event `self.EndLocation.OnComponentBeginOverlap`
  (params (OverlappedComponent :type "PrimitiveComponent Object Reference") (OtherActor :type "Actor Object Reference") (OtherComp :type "PrimitiveComponent Object Reference") (OtherBodyIndex :type Integer) (bFromSweep :type Boolean) (SweepResult :type "HitResult Structure (by ref)"))
  (`self.K2_SetActorRotation` OtherActor (struct :`Yaw` -90.0) false))

(fn `OpenDoor`
  (`SceneComponent.K2_AddLocalOffset` (`self.Door`) (0.0 0.0 0.0) false false))

(fn `UserConstructionScript`)