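; BP_SquadLocation is a movable squad position marker that tracks an assigned squad root and can hold one assigned squad member.
; Each tick it feeds the player pawn's last movement input into its own CharacterMovement, so it moves in step with the player.
; If it drifts beyond a fixed distance from a valid squad root, it teleports to that root's location and rotation.
; A ResetAssignedMember event clears the assigned member.
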(event `self.ReceiveTick`
  (params (DeltaSeconds :type "Float (single-precision)"))
  (bind _assignedsquadroot (`self.AssignedSquadRoot`))
  (`PawnMovementComponent.AddInputVector` (`self.CharacterMovement`) (`self.GetLastMovementInputVector` (`GameplayStatics.GetPlayerPawn` 0)) false)
  (`/Engine/EditorBlueprintResources/StandardMacros.IsValid` _assignedsquadroot
    (:`Is Valid`
      (if (>= (`self.GetDistanceTo` _assignedsquadroot self) 1250.0)
        (`self.K2_TeleportTo` self (`self.K2_GetActorLocation` _assignedsquadroot) (`self.K2_GetActorRotation` _assignedsquadroot))))))

(event `SquadInterface.ResetAssignedMember`
  (set `self.AssignedSquadMember` null))

(fn `UserConstructionScript`)